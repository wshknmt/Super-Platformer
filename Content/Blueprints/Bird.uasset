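; Flying eagle enemy that patrols along X, fires bullets and damages the player on box overlap.
; After a start delay, a Timeline drives the sprite's position and yaw, while a random Delay in its update paces Bullet spawns aimed along the facing direction.
; Overlapping the kill point while visible bounces the player upward and kills the bird, swapping hit and dead sprites and playing a screech before destroying it.
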(event `self.ReceiveBeginPlay`
  (bind _returnvalue (`self.GetTransform`))
  (bind (_returnvalue_x _returnvalue_y _returnvalue_z) (`KismetMathLibrary.BreakVector` (`SceneComponent.K2_GetComponentLocation` (`self.01_eagle_fly`))))
  (bind _returnvalue_2 (+ _returnvalue_z -9.0))
  (`KismetSystemLibrary.Delay` (`self.Delay`))
  (bind (_direction _position _rotate) (`Timeline|Timeline_0`)
    (:`Update`
      (bind _returnvalue_3 (== _rotate 0.0))
      (if _returnvalue_3
        (set `self.SpawnPositionX` (`KismetMathLibrary.MakeTransform` (`KismetMathLibrary.MakeVector` (+ _returnvalue_x 27.0) _returnvalue_y _returnvalue_2) (.rotation _returnvalue) (.scale _returnvalue)))
        (else
          (set `self.SpawnPositionX` (`KismetMathLibrary.MakeTransform` (`KismetMathLibrary.MakeVector` (+ _returnvalue_x -27.0) _returnvalue_y _returnvalue_2) (.rotation _returnvalue) (.scale _returnvalue)))))
      (if (not (`self.Dead`))
        (`SceneComponent.K2_SetRelativeLocationAndRotation` (`self.01_eagle_fly`) (`KismetMathLibrary.MakeVector` (* _position (`self.Range`))) (`KismetMathLibrary.MakeRotator` 0.0 0.0 _rotate) false false)
        (`KismetSystemLibrary.Delay` (`KismetMathLibrary.RandomFloatInRange` 0.8 2.0))
        (bind _returnvalue_4 (`|SpawnActorFromClass` "/Game/Blueprints/Bullet.Bullet_C" (`self.SpawnPositionX`) "Undefined" "OverrideRootScale" null null))
        (if _returnvalue_3
          (set `/Game/Blueprints/Bullet.Direction` 1.0 _returnvalue_4)
          (else
            (set `/Game/Blueprints/Bullet.Direction` -1.0 _returnvalue_4)))))))

(event `self.BoxCollision.OnComponentBeginOverlap`
  (params (OverlappedComponent :type "PrimitiveComponent Object Reference") (OtherActor :type "Actor Object Reference") (OtherComp :type "PrimitiveComponent Object Reference") (OtherBodyIndex :type Integer) (bFromSweep :type Boolean) (SweepResult :type "HitResult Structure (by ref)"))
  (if (`self.ActorHasTag` OtherActor "Player")
    (if (not (`self.Dead`))
      (bind _ascharacter (cast `/Game/Blueprints/Character` (`GameplayStatics.GetPlayerCharacter` 0)))
      (`/Game/Blueprints/Character.Take damage` _ascharacter))))

(event `self.Kill_point.OnComponentBeginOverlap`
  (params (OverlappedComponent :type "PrimitiveComponent Object Reference") (OtherActor :type "Actor Object Reference") (OtherComp :type "PrimitiveComponent Object Reference") (OtherBodyIndex :type Integer) (bFromSweep :type Boolean) (SweepResult :type "HitResult Structure (by ref)"))
  (if (`self.ActorHasTag` OtherActor "Player")
    (bind _ascharacter (cast `/Game/Blueprints/Character` (`GameplayStatics.GetPlayerCharacter` 0)))
    (if (not (`/Game/Blueprints/Character.IsInvisible` _ascharacter))
      (set `self.Dead` true)
      (bind _ascharacter_2 (cast `/Game/Blueprints/Character` (`GameplayStatics.GetPlayerCharacter` 0)))
      (`Character.LaunchCharacter` _ascharacter_2 (`KismetMathLibrary.MakeVector` 0.0 0.0 (* (`CharacterMovementComponent.JumpZVelocity` (`Character.CharacterMovement` _ascharacter_2)) 1.3)) false false)
      (`PrimitiveComponent.SetCollisionEnabled` (`self.Kill_point`) "NoCollision")
      (`SceneComponent.SetVisibility` (`self.01_eagle_fly`) false false)
      (`SceneComponent.SetVisibility` (`self.04_eagle_get_hit_Sprite`) true false)
      (`KismetSystemLibrary.Delay` 0.2)
      (`SceneComponent.SetVisibility` (`self.04_eagle_get_hit_Sprite`) false false)
      (`SceneComponent.SetVisibility` (`self.05_eagle_dead_Sprite`) true false)
      (`GameplayStatics.PlaySound2D` "/Game/Assety/Free/Enemy/Bird/mixkit-jungle-bird-screech-311.mixkit-jungle-bird-screech-311" 1.0 1.0 0.0 null null)
      (`KismetSystemLibrary.Delay` 0.2)
      (`self.K2_DestroyActor`))))

(fn `UserConstructionScript`)