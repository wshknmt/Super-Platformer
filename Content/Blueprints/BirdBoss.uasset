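; Eagle boss that flies a timeline-driven path, fires bullets, hurts the player on contact and shows a win screen when killed.
; Randomized Delays inside timeline updates pace the shots.
; As health drops, an Angle timeline rotates the aim and volleys grow from one bullet to two, then four.
; Kill-point overlaps by a visible player damage it, launch the player upward, update BossHealth and grant the boss brief invulnerability.
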(event `self.ReceiveBeginPlay`
  (bind _returnvalue (`self.GetTransform`))
  (bind _health (`self.Health`))
  (bind (_returnvalue_x _returnvalue_y _returnvalue_z) (`KismetMathLibrary.BreakVector` (`SceneComponent.K2_GetComponentLocation` (`self.01_eagle_fly`))))
  (bind _returnvalue_2 (+ _returnvalue_z -15.0))
  (`KismetSystemLibrary.Delay` (`self.Delay`))
  (bind (_direction _position _rotate) (`Timeline|Timeline_0`)
    (:`Update`
      (bind (_direction_2 _height) (`Timeline|HeightTimeline`)
        (:`Update`
          (bind _returnvalue_3 (== _rotate 0.0))
          (if _returnvalue_3
            (set `self.SpawnPositionX` (`KismetMathLibrary.MakeTransform` (`KismetMathLibrary.MakeVector` (+ _returnvalue_x 27.0) _returnvalue_y _returnvalue_2) (.rotation _returnvalue) (.scale _returnvalue)))
            (else
              (set `self.SpawnPositionX` (`KismetMathLibrary.MakeTransform` (`KismetMathLibrary.MakeVector` (+ _returnvalue_x -27.0) _returnvalue_y _returnvalue_2) (.rotation _returnvalue) (.scale _returnvalue)))))
          (if (not (`self.Dead`))
            (`SceneComponent.K2_SetRelativeLocationAndRotation` (`self.01_eagle_fly`) (`KismetMathLibrary.MakeVector` (* _position (`self.Range`)) 0.0 (* _height (`self.RangeHeight`))) (`KismetMathLibrary.MakeRotator` 0.0 0.0 _rotate) false false)
            (if (> (`self.Health`) 80.0)
              (`KismetSystemLibrary.Delay` (`KismetMathLibrary.RandomFloatInRange` 0.6 1.0))
              (else
                (bind (_direction_3 _angle) (`Timeline|Angle`)
                  (:`Update`
                    (if (> (`self.Health`) 60.0)
                      (`KismetSystemLibrary.Delay` (`KismetMathLibrary.RandomFloatInRange` 0.2 0.4))
                      (elif (> (`self.Health`) 40.0)
                        (`KismetSystemLibrary.Delay` (`KismetMathLibrary.RandomFloatInRange` 0.3 0.5))
                        (elif (> (`self.Health`) 20.0)
                          (`KismetSystemLibrary.Delay` (`KismetMathLibrary.RandomFloatInRange` 0.3 0.6))
                          (else
                            (`KismetSystemLibrary.Delay` (`KismetMathLibrary.RandomFloatInRange` 0.3 0.4))))))))))
            (if (not (`self.Dead`))
              (bind _returnvalue_4 (`|SpawnActorFromClass` "/Game/Blueprints/Bullet.Bullet_C" (`self.SpawnPositionX`) "Undefined" "OverrideRootScale" null null))
              (if (not (> _health 80.0))
                (bind _returnvalue_5 (`|SpawnActorFromClass` "/Game/Blueprints/Bullet.Bullet_C" (`self.SpawnPositionX`) "Undefined" "OverrideRootScale" null null))
                (set `/Game/Blueprints/Bullet.Rotation` (+ _angle 180.0) _returnvalue_5)
                (if _returnvalue_3
                  (set `/Game/Blueprints/Bullet.Direction` 1.0 _returnvalue_5)
                  (else
                    (set `/Game/Blueprints/Bullet.Direction` -1.0 _returnvalue_5)))
                (if (>= 40.0 _health)
                  (bind _returnvalue_6 (`|SpawnActorFromClass` "/Game/Blueprints/Bullet.Bullet_C" (`self.SpawnPositionX`) "Undefined" "OverrideRootScale" null null))
                  (set `/Game/Blueprints/Bullet.Rotation` (+ _angle 90.0) _returnvalue_6)
                  (if true
                    (set `/Game/Blueprints/Bullet.Direction` 1.0 _returnvalue_6)
                    (else
                      (set `/Game/Blueprints/Bullet.Direction` -1.0 _returnvalue_6)))
                  (bind _returnvalue_7 (`|SpawnActorFromClass` "/Game/Blueprints/Bullet.Bullet_C" (`self.SpawnPositionX`) "Undefined" "OverrideRootScale" null null))
                  (set `/Game/Blueprints/Bullet.Rotation` (+ _angle 270.0) _returnvalue_7)
                  (if true
                    (set `/Game/Blueprints/Bullet.Direction` 1.0 _returnvalue_7)
                    (else
                      (set `/Game/Blueprints/Bullet.Direction` -1.0 _returnvalue_7)))))
              (set `/Game/Blueprints/Bullet.Rotation` _angle _returnvalue_4)
              (if _returnvalue_3
                (set `/Game/Blueprints/Bullet.Direction` 1.0 _returnvalue_4)
                (else
                  (set `/Game/Blueprints/Bullet.Direction` -1.0 _returnvalue_4))))))))))

(event `self.BoxCollisionBoss.OnComponentBeginOverlap`
  (params (OverlappedComponent :type "PrimitiveComponent Object Reference") (OtherActor :type "Actor Object Reference") (OtherComp :type "PrimitiveComponent Object Reference") (OtherBodyIndex :type Integer) (bFromSweep :type Boolean) (SweepResult :type "HitResult Structure (by ref)"))
  (if (`self.ActorHasTag` OtherActor "Player")
    (if (not (`self.Dead`))
      (bind _ascharacter (cast `/Game/Blueprints/Character` (`GameplayStatics.GetPlayerCharacter` 0)))
      (`/Game/Blueprints/Character.Take damage` _ascharacter))))

(event `self.Kill_pointBoss.OnComponentBeginOverlap`
  (params (OverlappedComponent :type "PrimitiveComponent Object Reference") (OtherActor :type "Actor Object Reference") (OtherComp :type "PrimitiveComponent Object Reference") (OtherBodyIndex :type Integer) (bFromSweep :type Boolean) (SweepResult :type "HitResult Structure (by ref)"))
  (bind _returnvalue (- (`self.Health`) 15.0))
  (if (`self.ActorHasTag` OtherActor "Player")
    (bind _ascharacter (cast `/Game/Blueprints/Character` (`GameplayStatics.GetPlayerCharacter` 0)))
    (if (`/Game/Blueprints/Character.IsInvisible` _ascharacter)
      _
      (elif (not (`self.Invisible`))
        (set `self.Invisible` true)
        (`GameplayStatics.PlaySound2D` "/Game/Assety/Free/Enemy/Bird/mixkit-jungle-bird-screech-311.mixkit-jungle-bird-screech-311" 1.0 1.0 0.0 null null)
        (bind _ascharacter_2 (cast `/Game/Blueprints/Character` (`GameplayStatics.GetPlayerCharacter` 0)))
        (set `/Game/Blueprints/Character.Boss_Health` _returnvalue _ascharacter_2)
        (set `self.Health` _returnvalue)
        (`Character.LaunchCharacter` _ascharacter_2 (`KismetMathLibrary.MakeVector` 0.0 0.0 (* (`CharacterMovementComponent.JumpZVelocity` (`Character.CharacterMovement` _ascharacter_2)) 1.3)) false false)
        (`PrimitiveComponent.SetCollisionEnabled` (`self.Kill_pointBoss`) "NoCollision")
        (if (>= 0.0 (`self.Health`))
          (`SceneComponent.SetVisibility` (`self.01_eagle_fly`) false false)
          (`SceneComponent.SetVisibility` (`self.04_eagle_get_hit_Sprite`) true false)
          (`KismetSystemLibrary.Delay` 0.2)
          (`SceneComponent.SetVisibility` (`self.04_eagle_get_hit_Sprite`) false false)
          (`SceneComponent.SetVisibility` (`self.05_eagle_dead_Sprite`) true false)
          (`KismetSystemLibrary.Delay` 0.2)
          (`SceneComponent.SetVisibility` (`self.01_eagle_fly`) false true)
          (set `self.Dead` true)
          (`KismetSystemLibrary.Delay` 1.0)
          (bind _returnvalue_2 (`|CreateWidget` "/Game/Widgets/WinWidget1.WinWidget1_C"))
          (`UserWidget.AddToViewport` _returnvalue_2 0)
          (`GameplayStatics.SetGamePaused` true)
          (set `PlayerController.bShowMouseCursor` true (`GameplayStatics.GetPlayerController` 0))
          (`GameplayStatics.PlaySound2D` "/Game/Assety/Free/Items/tada-fanfare-a-6313.tada-fanfare-a-6313" 1.0 1.0 0.0 null null)
          (else
            (`KismetSystemLibrary.Delay` 1.0)
            (set `self.Invisible` false)
            (`PrimitiveComponent.SetCollisionEnabled` (`self.Kill_pointBoss`) "QueryAndPhysics")))))))

(fn `UserConstructionScript`)