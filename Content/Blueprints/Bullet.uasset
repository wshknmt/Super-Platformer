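; Bullet projectile actor that flies in a straight line in the X-Z plane and damages the player.
; A timeline started on BeginPlay offsets the sprite by Range along the Rotation angle, with Direction scaling the X component.
; A delay triggered from the timeline update destroys the actor after four seconds.
; Overlapping a Player-tagged actor calls TakeDamage on player character 0, without destroying the bullet.
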(event `self.ReceiveBeginPlay`
  (bind _rotation (`self.Rotation`))
  (bind (_direction _position) (`Timeline|Timeline_0`)
    (:`Update`
      (bind _returnvalue (* _position (`self.Range`)))
      (`SceneComponent.K2_SetRelativeLocationAndRotation` (`self.projectile_1_Sprite`) (`KismetMathLibrary.MakeVector` (* (* _returnvalue (`KismetMathLibrary.DegCos` _rotation)) (`self.Direction`)) 0.0 (* _returnvalue (`KismetMathLibrary.DegSin` _rotation))) (`KismetMathLibrary.MakeRotator` 0.0) false false)
      (`KismetSystemLibrary.Delay` 4.0)
      (`self.K2_DestroyActor`))))

(event `self. Collision box.OnComponentBeginOverlap`
  (params (OverlappedComponent :type "PrimitiveComponent Object Reference") (OtherActor :type "Actor Object Reference") (OtherComp :type "PrimitiveComponent Object Reference") (OtherBodyIndex :type Integer) (bFromSweep :type Boolean) (SweepResult :type "HitResult Structure (by ref)"))
  (if (`self.ActorHasTag` OtherActor "Player")
    (bind _ascharacter (cast `/Game/Blueprints/Character` (`GameplayStatics.GetPlayerCharacter` 0)))
    (`/Game/Blueprints/Character.Take damage` _ascharacter)))

(fn `UserConstructionScript`)