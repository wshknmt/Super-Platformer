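; Coin pickup actor, drawn with a flipbook, that the player collects by touching it.
; A sphere overlap with an actor tagged "Player" destroys the coin and plays a 2D notification sound.
; It then calls EarnCoin on player 0's character, fetched by index and cast rather than taken from the overlapping actor.
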(event `self.Sphere.OnComponentBeginOverlap`
  (params (OverlappedComponent :type "PrimitiveComponent Object Reference") (OtherActor :type "Actor Object Reference") (OtherComp :type "PrimitiveComponent Object Reference") (OtherBodyIndex :type Integer) (bFromSweep :type Boolean) (SweepResult :type "HitResult Structure (by ref)"))
  (if (`self.ActorHasTag` OtherActor "Player")
    (cast `/Game/Blueprints/Character` (`GameplayStatics.GetPlayerCharacter` 0))
    (`self.K2_DestroyActor` (`ActorComponent.GetOwner` (`self.coin_flipbook`)))
    (`GameplayStatics.PlaySound2D` "/Game/Assety/Free/Items/Coins/mixkit-unlock-game-notification-253.mixkit-unlock-game-notification-253" 1.0 1.0 0.0 null null)
    (bind _ascharacter (cast `/Game/Blueprints/Character` (`GameplayStatics.GetPlayerCharacter` 0)))
    (`/Game/Blueprints/Character.Earn coin` _ascharacter)))

(fn `UserConstructionScript`)