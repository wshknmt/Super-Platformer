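; A level-exit door that unlocks once the player has collected the maximum coin count and leads to the boss level.
; BeginPlay disables the box collision and starts a timeline, whose updates compare the player character's coins to its maximum.
; When the count is met, the timeline update shows the wooden door sprite and enables query-only collision.
; Overlapping the box opens BossLevel and sets game-only input mode.
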(event `self.ReceiveBeginPlay`
  (`PrimitiveComponent.SetCollisionEnabled` (`self. Box collision`) "NoCollision")
  (`Timeline|Timeline_0`
    (:`Update`
      (bind _ascharacter (cast `/Game/Blueprints/Character` (`GameplayStatics.GetPlayerCharacter` 0)))
      (if (>= (`/Game/Blueprints/Character.Coins` _ascharacter) (`/Game/Blueprints/Character.MAX_COINS` _ascharacter))
        (`SceneComponent.SetVisibility` (`self.Wooden_Door_Sprite_0`) true false)
        (`PrimitiveComponent.SetCollisionEnabled` (`self. Box collision`) "QueryOnly")))))

(event `self. Box collision.OnComponentBeginOverlap`
  (params (OverlappedComponent :type "PrimitiveComponent Object Reference") (OtherActor :type "Actor Object Reference") (OtherComp :type "PrimitiveComponent Object Reference") (OtherBodyIndex :type Integer) (bFromSweep :type Boolean) (SweepResult :type "HitResult Structure (by ref)"))
  (`GameplayStatics.OpenLevelBySoftObjectPtr` "/Game/Mapy/BossLevel.BossLevel")
  (`WidgetBlueprintLibrary.SetInputMode_GameOnly` (`GameplayStatics.GetPlayerController` 0)))

(fn `UserConstructionScript`)