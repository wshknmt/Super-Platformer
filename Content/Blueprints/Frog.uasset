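; Frog is an actor that tells the player whether enough coins have been collected to unlock a level.
; When its box collision begins an overlap, it casts player 0's pawn to Character and compares Coins against MAXCOINS.
; It shows the LevelUnlocked sprite if the count is met, otherwise a second text sprite, and hides both when the overlap ends.
; The overlapping actor is never checked, and the Blueprint only displays the result.
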(event `self. Box Collision.OnComponentBeginOverlap`
  (params (OverlappedComponent :type "PrimitiveComponent Object Reference") (OtherActor :type "Actor Object Reference") (OtherComp :type "PrimitiveComponent Object Reference") (OtherBodyIndex :type Integer) (bFromSweep :type Boolean) (SweepResult :type "HitResult Structure (by ref)"))
  (bind _ascharacter (cast `/Game/Blueprints/Character` (`GameplayStatics.GetPlayerCharacter` 0)))
  (if (>= (`/Game/Blueprints/Character.Coins` _ascharacter) (`/Game/Blueprints/Character.MAX_COINS` _ascharacter))
    (`SceneComponent.SetVisibility` (`self.levelUnlocked_Sprite`) true false)
    (else
      (`SceneComponent.SetVisibility` (`self.cooltext428148843874419_Sprite`) true false))))

(event `self. Box Collision.OnComponentEndOverlap`
  (params (OverlappedComponent :type "PrimitiveComponent Object Reference") (OtherActor :type "Actor Object Reference") (OtherComp :type "PrimitiveComponent Object Reference") (OtherBodyIndex :type Integer))
  (`SceneComponent.SetVisibility` (`self.cooltext428148843874419_Sprite`) false false)
  (`SceneComponent.SetVisibility` (`self.levelUnlocked_Sprite`) false false))

(fn `UserConstructionScript`)