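; HeartSpawner is a respawning health pickup shown as a heart flipbook with a sphere trigger.
; When an actor tagged Player overlaps the sphere, it calls IncreaseHealth on the first player's character and plays a 2D sound.
; It then disables the sphere's collision and hides the heart, restoring both after the SpawnTime delay instead of destroying or spawning actors.
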(event `self.Sphere.OnComponentBeginOverlap`
  (params (OverlappedComponent :type "PrimitiveComponent Object Reference") (OtherActor :type "Actor Object Reference") (OtherComp :type "PrimitiveComponent Object Reference") (OtherBodyIndex :type Integer) (bFromSweep :type Boolean) (SweepResult :type "HitResult Structure (by ref)"))
  (if (`self.ActorHasTag` OtherActor "Player")
    (bind _ascharacter (cast `/Game/Blueprints/Character` (`GameplayStatics.GetPlayerCharacter` 0)))
    (`/Game/Blueprints/Character.Increase health` _ascharacter)
    (`GameplayStatics.PlaySound2D` "/Game/Assety/Free/Heart/heartEffect.heartEffect" 1.0 1.0 0.0 null null)
    (`PrimitiveComponent.SetCollisionEnabled` (`self.Sphere`) "NoCollision")
    (`SceneComponent.SetVisibility` (`self.HeartFlipbook`) false false)
    (`KismetSystemLibrary.Delay` (`self.SpawnTime`))
    (`PrimitiveComponent.SetCollisionEnabled` (`self.Sphere`) "QueryAndPhysics")
    (`SceneComponent.SetVisibility` (`self.HeartFlipbook`) true false)))

(fn `UserConstructionScript`)