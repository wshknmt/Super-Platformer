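; Hiena is a hyena enemy that patrols with flipbook sprites and can be killed by the player.
; After a start delay, a timeline drives the walk sprite's X offset, scaled by Range, and its yaw until death.
; Body overlap damages the player while the hyena lives.
; Kill point overlap, unless the player is invisible, bounces the player upward, swaps to the death flipbook, plays a howl and destroys the actor after a delay.
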(event `self.ReceiveBeginPlay`
  (`KismetSystemLibrary.Delay` (`self.Delay`))
  (bind (_direction _position _rotate) (`Timeline|HienaTimeline`)
    (:`Update`
      (if (not (`self.Dead`))
        (`SceneComponent.K2_SetRelativeLocationAndRotation` (`self.Hyena_walk1_Flipbook`) (`KismetMathLibrary.MakeVector` (* _position (`self.Range`))) (`KismetMathLibrary.MakeRotator` 0.0 0.0 _rotate) false false)))))

(event `self.  Box_collision.OnComponentBeginOverlap`
  (params (OverlappedComponent :type "PrimitiveComponent Object Reference") (OtherActor :type "Actor Object Reference") (OtherComp :type "PrimitiveComponent Object Reference") (OtherBodyIndex :type Integer) (bFromSweep :type Boolean) (SweepResult :type "HitResult Structure (by ref)"))
  (if (`self.ActorHasTag` OtherActor "Player")
    (if (not (`self.Dead`))
      (bind _ascharacter (cast `/Game/Blueprints/Character` (`GameplayStatics.GetPlayerCharacter` 0)))
      (`/Game/Blueprints/Character.Take damage` _ascharacter))))

(event `self.Kill_point.OnComponentBeginOverlap`
  (params (OverlappedComponent :type "PrimitiveComponent Object Reference") (OtherActor :type "Actor Object Reference") (OtherComp :type "PrimitiveComponent Object Reference") (OtherBodyIndex :type Integer) (bFromSweep :type Boolean) (SweepResult :type "HitResult Structure (by ref)"))
  (if (`self.ActorHasTag` OtherActor "Player")
    (bind _ascharacter (cast `/Game/Blueprints/Character` (`GameplayStatics.GetPlayerCharacter` 0)))
    (if (not (`/Game/Blueprints/Character.IsInvisible` _ascharacter))
      (set `self.Dead` true)
      (bind _ascharacter_2 (cast `/Game/Blueprints/Character` (`GameplayStatics.GetPlayerCharacter` 0)))
      (`Character.LaunchCharacter` _ascharacter_2 (`KismetMathLibrary.MakeVector` 0.0 0.0 (* (`CharacterMovementComponent.JumpZVelocity` (`Character.CharacterMovement` _ascharacter_2)) 1.3)) false false)
      (`PrimitiveComponent.SetCollisionEnabled` (`self.Kill_point`) "NoCollision")
      (`SceneComponent.SetVisibility` (`self.Hyena_walk1_Flipbook`) false false)
      (`SceneComponent.SetVisibility` (`self.HyenaDeadFlipbook`) true false)
      (`GameplayStatics.PlaySound2D` "/Game/Assety/Free/Enemy/Hyena/mixkit-cartoon-wolf-howling-1774.mixkit-cartoon-wolf-howling-1774" 1.0 1.0 0.0 null null)
      (`KismetSystemLibrary.Delay` 1.0)
      (`self.K2_DestroyActor`))))

(fn `UserConstructionScript`)