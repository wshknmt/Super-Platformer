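; Jump pad actor that launches the player upward when they overlap its box trigger.
; After a brief delay, it launches player character 0 with a Z velocity of its jump velocity scaled by LaunchStrength and plays a spring sound.
; It then briefly swaps the JumpPad visual for a jump flipbook before restoring it.
; Only actors tagged Player trigger it.
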(event `self.Box.OnComponentBeginOverlap`
  (params (OverlappedComponent :type "PrimitiveComponent Object Reference") (OtherActor :type "Actor Object Reference") (OtherComp :type "PrimitiveComponent Object Reference") (OtherBodyIndex :type Integer) (bFromSweep :type Boolean) (SweepResult :type "HitResult Structure (by ref)"))
  (if (`self.ActorHasTag` OtherActor "Player")
    (bind _ascharacter (cast `/Game/Blueprints/Character` (`GameplayStatics.GetPlayerCharacter` 0)))
    (`KismetSystemLibrary.Delay` 0.15)
    (`Character.LaunchCharacter` _ascharacter (`KismetMathLibrary.MakeVector` 0.0 0.0 (* (`CharacterMovementComponent.JumpZVelocity` (`Character.CharacterMovement` _ascharacter)) (`self.LaunchStrength`))) false false)
    (`GameplayStatics.PlaySound2D` "/Game/Assety/Free/Traps/Trampoline/zapsplat_cartoon_springing_boing_jump_jaw_harp_006_72951.zapsplat_cartoon_springing_boing_jump_jaw_harp_006_72951" 1.0 1.0 0.0 null null)
    (`SceneComponent.SetVisibility` (`self.Jump_FLIPBOOK_28x28`) true false)
    (`SceneComponent.SetVisibility` (`self.JumpPad`) false false)
    (`KismetSystemLibrary.Delay` 0.5)
    (`SceneComponent.SetVisibility` (`self.Jump_FLIPBOOK_28x28`) false false)
    (`SceneComponent.SetVisibility` (`self.JumpPad`) true false)))

(fn `UserConstructionScript`)